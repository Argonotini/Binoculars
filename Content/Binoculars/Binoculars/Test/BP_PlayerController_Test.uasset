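; Test player controller that manages the binoculars UI widget.
; Four custom events create, show, hide and destroy a WB_Binoculars_Test widget held in GUIBinoculars, with validity checks before showing, hiding or destroying it.
; Hide only removes the widget from its parent, keeping the instance for reuse, while destroy also clears the reference.
; RetrieveCameraComponent and RetrieveCameraZoom are stubs that return empty or zero values.
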(event `CreateBinoculars_1`
  ;[0 0 0] Binoculars
  (bind _returnvalue (`|CreateWidget` "/Game/Binoculars/Binoculars/Test/WB_Binoculars_Test.WB_Binoculars_Test_C"))
  (set `self.GUI_Binoculars` _returnvalue))

(event `DestroyBinoculars_1`
  ;[0 0 0] Binoculars
  (`/Engine/EditorBlueprintResources/StandardMacros.IsValid` (`self.GUI_Binoculars`)
    (:`Is Valid`
      (`Widget.RemoveFromParent` (`self.GUI_Binoculars`))
      (set `self.GUI_Binoculars` null))))

(event `ShowBinoculars_1`
  ;[0 0 0] Binoculars
  (`/Engine/EditorBlueprintResources/StandardMacros.IsValid` (`self.GUI_Binoculars`)
    (:`Is Valid`
      (`UserWidget.AddToViewport` (`self.GUI_Binoculars`) 0))))

(event `HideBinoculars_1`
  ;[0 0 0] Binoculars
  (`/Engine/EditorBlueprintResources/StandardMacros.IsValid` (`self.GUI_Binoculars`)
    (:`Is Valid`
      (`Widget.RemoveFromParent` (`self.GUI_Binoculars`)))))

(fn `RetrieveCameraComponent`
  (returns (CameraComponent :type "CameraComponent Object Reference"))
  (return null))

(fn `RetrieveCameraZoom`
  (returns (CameraZoom :type "Float (double-precision)"))
  (return 0.0))

(fn `UserConstructionScript`)