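; BP_PlayerHUD is the player's HUD, drawing a centered crosshair texture and managing the binoculars overlay.
; It sets game-only input on BeginPlay and draws the crosshair directly in DrawHUD.
; Equip and unequip events create or remove a WB_BinocularsVision widget, initialized with the current zoom factor.
; A zoom-modified event forwards new factors to that widget while it is valid.
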(event `self.ReceiveBeginPlay`
  (`WidgetBlueprintLibrary.SetInputMode_GameOnly` (`GameplayStatics.GetPlayerController` 0)))

(event `self.ReceiveDrawHUD`
  (params (SizeX :type Integer) (SizeY :type Integer))
  ;[0 0 0] Нарисуйте перекрестие в центре экрана
  (`self.DrawTexture` "/Game/Binoculars/Binoculars/Texture/T_Crosshair.T_Crosshair" (`KismetMathLibrary.Conv_IntToDouble` (- (/ SizeX 2) 8)) (`KismetMathLibrary.Conv_IntToDouble` (- (/ SizeY 2) 8)) 16.0 16.0 0.0 0.0 1.0 1.0 (make `LinearColor` 1.0 1.0 1.0 1.0) "BLEND_Translucent" 1.0 true))

(event `OnBinocularsEquipped`
  (params (ZoomFactor :type "Float (double-precision)"))
  ;[0 0 0] Изменения HUD, связанные с экипировкой/снятием биноклей
  (bind _returnvalue (`|CreateWidget` "/Game/Binoculars/Binoculars/UI/BinocularsView/WB_BinocularsVision.WB_BinocularsVision_C" null ZoomFactor))
  (bind _output_get (set `self.BinocularsWidget` _returnvalue))
  (`UserWidget.AddToViewport` _output_get 0))

(event `OnBinocularsUnequipped`
  ;[0 0 0] Изменения HUD, связанные с экипировкой/снятием биноклей
  (`/Engine/EditorBlueprintResources/StandardMacros.IsValid` (`self.BinocularsWidget`)
    (:`Is Valid`
      (`Widget.RemoveFromParent` (`self.BinocularsWidget`))
      (set `self.BinocularsWidget` null))))

(event `OnBinocularsZoomFactorModified`
  (params (ZoomFactor :type "Float (double-precision)"))
  ;[0 0 0] Используйте для обновления HUD при изменении коэффициента масштабирования.
  (`/Engine/EditorBlueprintResources/StandardMacros.IsValid` (`self.BinocularsWidget`)
    (:`Is Valid`
      (`/Game/Binoculars/Binoculars/UI/BinocularsView/WB_BinocularsVision.UpdateZoomValue` (`self.BinocularsWidget`) ZoomFactor))))

(fn `UserConstructionScript`)