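; BP_Tag_WC is a widget component that shows a toggleable binoculars tag on its owning actor, displaying range to the player.
; Toggling shows or hides the widget, plays a UI sound, and starts or clears a looping update timer.
; Each update writes distance in metres to WB_Binoculars_Tag and offsets the component from its default position using camera-zoom-adjusted distance, keeping it just above the owner.
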(event Custom|OnChangeTagState
  (if (Variables|RuntimeAllocation|GetIsEnabled?)
    ;[0 0 0] Деактивация тега
    (Widget|SetVisibility (UserInterface|GetUserWidgetObject) "Hidden")
    (Utilities|Time|ClearandInvalidateTimerbyHandle (Variables|TimerHandles|GetWidgetUpdateTimer))
    (Components|Tick|SetComponentTickEnabled true)
    (Variables|RuntimeAllocation|SetIsEnabled? false)
    (Audio|PlaySound2D "/Engine/VREditor/Sounds/UI/Floating_UI_Close.Floating_UI_Close" 1.0 1.0 0.0 0 0)
    (else
      ;[0 0 0] Активация тега
      (Variables|RuntimeAllocation|SetIsEnabled? true)
      (CallFunction|OnBeginUpdate) ; Немедленно выполняет первый цикл обновления
      (Components|Tick|SetComponentTickEnabled true)
      (bind _returnvalue (Utilities|Time|SetTimerbyEvent (delegate Custom|OnBeginUpdate) (Variables|Config|GetWidgetUpdateTimerInterval) true)) ; Запускает таймер для обновления состояния виджета
      (Variables|TimerHandles|SetWidgetUpdateTimer _returnvalue)
      (Widget|SetVisibility (UserInterface|GetUserWidgetObject) "Visible")
      (Audio|PlaySound2D "/Engine/VREditor/Sounds/VR_click1.VR_click1" 1.0 1.0 0.0 0 0))))

(event Custom|OnBeginUpdate
  ;[0 0 0] Обновляет состояние виджета
  (bind _aswb_binoculars_tag (Utilities|Casting|CastToWB_Binoculars_Tag (UserInterface|GetUserWidgetObject)))
  (Utilities|IsValid (Game|Player|GetPlayerPawn 0)
    (:Is%20Valid
      (bind (_truedistance _camzoomadjuste) (CallFunction|CalculateDistancefromPlayer))
      (Default|UpdateRangeText _aswb_binoculars_tag (/ _truedistance 1e+02))
      (Transformation|SetRelativeLocation (|(Origin+(Origin*(ZoomAdjustedDistance*LocationModifier))) (Variables|RuntimeAllocation|GetDefaultRelativeLocation) _camzoomadjuste (Variables|Config|GetRelativeLocationModifier)) false false) ; Обновляет относительное расположение виджета, чтобы гарантировать, что он всегда отображается чуть выше актера-владельца.
    )))

(event EventBeginPlay
  ;[0 0 0] Протоколы инициализации
  (Variables|RuntimeAllocation|SetDefaultRelativeLocation (Variables|Default|GetRelativeLocation)))

(fn CalculateDistancefromPlayer
  (LocalVariables|SetLocal_DistanceToPlayer (Transformation|GetDistanceTo (Components|GetOwner) (Game|Player|GetPlayerPawn 0)))
  (bind _camerazoom (Class|BPIPlayerCharacter|RetrieveCameraZoom(Message) (Game|Player|GetPlayerPawn 0)))
  (return (LocalVariables|GetLocal_DistanceToPlayer) (/ (LocalVariables|GetLocal_DistanceToPlayer) _camerazoom)))