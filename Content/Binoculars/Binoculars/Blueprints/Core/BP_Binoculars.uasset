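; BP_Binoculars is a child-actor binoculars item that lets its parent zoom the view and tag targets.
; Equip, unequip and zoom events play sounds, notify BP_PlayerHUD and set the parent camera's FOV, fetched through a message call.
; Clamped zoom factor converts to FOV via a tangent formula based on the default FOV.
; Tagging line-traces from the camera, calls the hit actor's BP_Tag_WC and enables skeletal-mesh custom depth for outlines.
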(event `self.ReceiveBeginPlay`
  ;[0 0 0 0.5] Протоколы инициализации
  (set `self.ZoomFactor` (`self.MinZoom`)) ; Устанавливает минимальное значение масштаба в качестве масштаба по умолчанию
  (bind _cameracomponent (message `/Game/Binoculars/Binoculars/Blueprints/Core/BPI_PlayerCharacter.RetrieveCameraComponent` (`self.GetParentActor`)))
  (set `self.DefaultFieldOfView` (`CameraComponent.FieldOfView` _cameracomponent)) ; Сохраняет поле зрения по умолчанию для компонента камеры родительского актера.
)

(event `OnEquipped`
  ;[0 0 0] Экипировать/снять логику
  (if (not (`self.Equipped?`))
    (set `self.Equipped?` true)
    (bind _asbp_player_hud (cast `/Game/Binoculars/Binoculars/Blueprints/Player/BP_PlayerHUD` (`PlayerController.GetHUD` (`GameplayStatics.GetPlayerController` 0))))
    (`/Game/Binoculars/Binoculars/Blueprints/Player/BP_PlayerHUD.OnBinocularsEquipped` _asbp_player_hud (`self.ZoomFactor`))
    (bind _fieldofview (`self.CalculateFoVForZoomValue` (`self.ZoomFactor`)))
    (`self.UpdateFoV` _fieldofview)
    (`GameplayStatics.PlaySound2D` "/Engine/VREditor/Sounds/UI/Click_on_Button_Cue.Click_on_Button_Cue" 1.0 1.0 0.0 null null)))

(event `OnUnequipped`
  ;[0 0 0] Экипировать/снять логику
  (if (`self.Equipped?`)
    (bind _asbp_player_hud (cast `/Game/Binoculars/Binoculars/Blueprints/Player/BP_PlayerHUD` (`PlayerController.GetHUD` (`GameplayStatics.GetPlayerController` 0))))
    (`/Game/Binoculars/Binoculars/Blueprints/Player/BP_PlayerHUD.OnBinocularsUnequipped` _asbp_player_hud)
    (`self.UpdateFoV` (`self.DefaultFieldOfView`))
    (set `self.Equipped?` false)
    (`GameplayStatics.PlaySound2D` "/Engine/EditorSounds/Notifications/CompileStart_Cue.CompileStart_Cue" 1.0 1.0 0.0 null null)))

(event `ZoomIn`
  ;[0 0 0] Логика увеличения/уменьшения
  (if (`self.Equipped?`)
    (`self.ModifyZoomFactor` (`self.ZoomStep`)) ; Increase zoom level
    (bind _fieldofview (`self.CalculateFoVForZoomValue` (`self.ZoomFactor`) :!label _label))
    (`self.UpdateFoV` _fieldofview)
    (`GameplayStatics.PlaySound2D` "/Engine/VREditor/Sounds/UI/Dockable_Window_Close.Dockable_Window_Close" 1.0 1.0 0.0 null null)))

(event `ZoomOut`
  ;[0 0 0] Логика увеличения/уменьшения
  (if (`self.Equipped?`)
    (`self.ModifyZoomFactor` (* (`self.ZoomStep`) -1.0)) ; Уменьшить уровень масштабирования
    (goto _label)))

(event `UpdateFoV`
  (params (NewFieldOfView :type "Float (double-precision)"))
  ;[0 0 0] Обновляет поле зрения компонента камеры родительского актера.
  (bind _cameracomponent (message `/Game/Binoculars/Binoculars/Blueprints/Core/BPI_PlayerCharacter.RetrieveCameraComponent` (`self.GetParentActor`)))
  (`CameraComponent.SetFieldOfView` _cameracomponent NewFieldOfView))

(fn `CalculateFoVForZoomValue`
  (params (ZoomFactor :type "Float (double-precision)"))
  (returns (FieldOfView :type "Float (double-precision)"))
  ;[0 0 0] Вычисляет поле зрения, связанное с уровнем масштабирования, по формуле: NewFoV = 2*atan(tan(DefaultFoV/2)/ZoomFactor)
  (return (* (`KismetMathLibrary.DegAtan` (/ (`KismetMathLibrary.DegTan` (/ (`self.DefaultFieldOfView`) 2.0)) ZoomFactor)) 2.0)))

(fn `GetZoomFactor`
  (returns (ZoomFactor :type "Float (double-precision)"))
  (return (`self.ZoomFactor`)))

(fn `IsEquipped?`
  (returns (`Yes?` :type Boolean))
  (return (`self.Equipped?`)))

(fn `ModifyZoomFactor`
  (params (Delta :type "Float (double-precision)"))
  ;[0 0 0] Изменяет коэффициент масштабирования на указанную дельту
  (set `self.ZoomFactor` (`KismetMathLibrary.FClamp` (+ (`self.ZoomFactor`) Delta) (`self.MinZoom`) (`self.MaxZoom`)))
  (bind _asbp_player_hud (cast `/Game/Binoculars/Binoculars/Blueprints/Player/BP_PlayerHUD` (`PlayerController.GetHUD` (`GameplayStatics.GetPlayerController` 0)))
    (:`then`
      (`/Game/Binoculars/Binoculars/Blueprints/Player/BP_PlayerHUD.OnBinocularsZoomFactorModified` _asbp_player_hud (`self.ZoomFactor`)))
    (:`CastFailed`
      _))
  (return))

(fn `TagTargetEnitity`
  ;[0 0 0] Отмечает объект, сфокусированный игроком
  (if (`self.Equipped?`)
    (bind _cameracomponent (message `/Game/Binoculars/Binoculars/Blueprints/Core/BPI_PlayerCharacter.RetrieveCameraComponent` (`self.GetParentActor`)))
    (bind _returnvalue (`SceneComponent.K2_GetComponentLocation` _cameracomponent))
    (bind _outhit (`KismetSystemLibrary.LineTraceSingle` _returnvalue (+ _returnvalue (* (`SceneComponent.GetForwardVector` _cameracomponent) (`self.MaxTaggingDistance`))) "TraceTypeQuery2" false (`|MakeArray` (`self.GetParentActor`))))
    (bind (_bblockinghit _binitialoverlap _time _distance _location _impactpoint _normal _impactnormal _physmat _hitactor) (`GameplayStatics.BreakHitResult` _outhit))
    (if _bblockinghit
      (bind _returnvalue_2 (`self.GetComponentByClass` _hitactor "/Game/Binoculars/Binoculars/Blueprints/Core/BP_Tag_WC.BP_Tag_WC_C"))
      (`/Engine/EditorBlueprintResources/StandardMacros.IsValid` _returnvalue_2
        (:`Is Valid`
          (`/Game/Binoculars/Binoculars/Blueprints/Core/BP_Tag_WC.OnChangeTagState` _returnvalue_2))
        (:`Is Not Valid`
          _))
      (for _array_element (`self.K2_GetComponentsByClass` _hitactor "/Script/Engine.SkeletalMeshComponent")
        (`/Engine/EditorBlueprintResources/StandardMacros.IsValid` _array_element
          (:`Is Valid`
            (`PrimitiveComponent.SetRenderCustomDepth` _array_element true) ; Запрашивает все компоненты скелетной сетки, принадлежащие цели попадания, для рендеринга с пользовательской глубиной (для контура).
          ))))))

(fn `UserConstructionScript`)